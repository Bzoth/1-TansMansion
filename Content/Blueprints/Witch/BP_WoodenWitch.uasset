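; AI witch enemy character that moves between dolls and switches among idle, search and chase states.
; State changes replicate via server and multicast events, updating the blackboard and walk speed, with a debug print.
; Cycling the doll index sets the blackboard move target to a random reachable point near that doll.
; It also plays a networked swing montage, gets launched by blows, and can be frozen inside a spawned ice prison.
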(event `self.ReceiveBeginPlay`
  (`KismetSystemLibrary.PrintString` (`|GetEnumeratorNameAsString` (`self.State`)) true true (struct :`R` 1.0 :`A` 1.0) 99999.0 "State"))

(event `IncreaseDollIndex`
  (bind _output_get (set `self.DollIndex` (+ (`self.DollIndex`) 1)))
  (if (>= _output_get (`KismetArrayLibrary.Array_Length` (`self.Dolls`)))
    (set `self.DollIndex` 0))
  (`BlackboardComponent.SetValueAsVector` (`AIBlueprintHelperLibrary.GetBlackboard` null) "MoveLocation" (`NavigationSystemV1.K2_GetRandomReachablePointInRadius` (`SceneComponent.K2_GetComponentLocation` (`/Game/Blueprints/Witch/BP_TestDoll.DefaultSceneRoot` (`|GetArrayItem` (`self.Dolls`) (`self.DollIndex`)))) 500.0 (`self.Nav Data`) null)))

(event `SwapState`
  (params (NewState :type "/Game/Blueprints/Witch/E_WitchState Enum" :default "NewEnumerator0"))
  (`self.S_SwapState` NewState))

(event `M_SwapState`
  (params (State :type "/Game/Blueprints/Witch/E_WitchState Enum" :default "NewEnumerator0"))
  (bind _returnvalue (`AIBlueprintHelperLibrary.GetBlackboard` self))
  (set `self.State` State)
  (`/Engine/EditorBlueprintResources/StandardMacros.IsValid` _returnvalue
    (:`Is Valid`
      (`BlackboardComponent.SetValueAsEnum` _returnvalue "State" (`self.State`))
      (`KismetSystemLibrary.PrintString` (`|GetEnumeratorNameAsString` (`self.State`)) true true (struct :`R` 1.0 :`A` 1.0) 99999.0 "State")
      (set `CharacterMovementComponent.MaxWalkSpeed` (select `/Game/Blueprints/Witch/E_WitchState` (`self.State`) :`NewEnumerator0` 75.0 :`NewEnumerator1` 250.0 :`NewEnumerator2` 600.0 :!type "Float (single-precision)") (`self.CharacterMovement`)))))

(event `S_SwapState`
  (params (State :type "/Game/Blueprints/Witch/E_WitchState Enum" :default "NewEnumerator0"))
  (`self.M_SwapState` State))

(event `SwingAttack`
  (`self.ServerPlayMontage` "/Game/Assets/Animations/AM_Witch_Attack_Montage.AM_Witch_Attack_Montage"))

(event `ServerPlayMontage`
  (params (MontageToPlay :type "AnimMontage Object Reference"))
  (`self.PlayMontage` MontageToPlay))

(event `PlayMontage`
  (params (MontageToPlay :type "AnimMontage Object Reference"))
  (`|PlayMontage` (`self.Mesh`) MontageToPlay))

(event `/Game/Blueprints/Management/BPI_Interract.BlowTarget`
  (params (BlowLocation :type "Vector Structure"))
  (`self.LaunchCharacter` (* (- (`self.K2_GetActorLocation`) BlowLocation) (25.0 25.0 12.0)) true)
  (`self.StopAnimMontage` (`self.GetCurrentMontage`))
  (`MovementComponent.StopMovementImmediately` (`self.CharacterMovement`)))

(event `/Game/Blueprints/Management/BPI_Interract.Freeze`
  (`|ExecutionSequence`
    (:`then_0`
      (set `CharacterMovementComponent.MaxWalkSpeed` 0.0 (`self.CharacterMovement`)))
    (:`then_1`
      (`self.S_Freeze`))))

(event `S_Freeze`
  (`self.M_Freeze`))

(event `M_Freeze`
  (bind _returnvalue (`|SpawnActorFromClass` "/Game/Blueprints/Spells/BP_IcePrison.BP_IcePrison_C" (`SceneComponent.K2_GetComponentToWorld` (`self.Mesh`)) "Undefined" "MultiplyWithRoot" null self null))
  (`/Game/Blueprints/Spells/BP_IcePrison.S_MeltPrison` _returnvalue))

(event `/Game/Blueprints/Management/BPI_Interract.DisableEverything`
  (params (Disable :type Boolean))
  (if (not Disable)
    (set `CharacterMovementComponent.MaxWalkSpeed` (select `/Game/Blueprints/Witch/E_WitchState` (`self.State`) :`NewEnumerator0` 75.0 :`NewEnumerator1` 250.0 :`NewEnumerator2` 600.0 :!type "Float (single-precision)") (`self.CharacterMovement`))))

(fn `GetFlamableType`
  (returns (Type :type "/Game/Blueprints/Management/E_FlameInterractable Enum"))
  (return "NewEnumerator2"))

(fn `Interract`
  (params (Interractor :type "Actor Object Reference"))
  (returns (Interractable :type "/Game/Blueprints/Interraction/BP_Interractable Object Reference"))
  (return null))

(fn `UserConstructionScript`)