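; AI controller for the wooden witch enemy that runs its behavior tree and escalates its state as it perceives stimuli.
; Each perception update adds stimulus strength to a noise meter through a server-named event.
; Any non-negative meter moves Idle to Search with a lock-on montage.
; Crossing a higher threshold moves Search to Chase with a shriek montage and writes the perceived actor to the blackboard as TargetPlayer.
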(event `self.ReceiveBeginPlay`
  (bind _asbp_wooden_witch (cast `/Game/Blueprints/Witch/BP_WoodenWitch` (`self.K2_GetPawn`)))
  (set `self.Witch` _asbp_wooden_witch)
  (`self.RunBehaviorTree` "/Game/Blueprints/Witch/BT_Witch.BT_Witch"))

(event `self.AIPerception.OnTargetPerceptionUpdated`
  (params (Actor :type "Actor Object Reference") (Stimulus :type "AIStimulus Structure"))
  (`self.ServerSetNoiseMeter` (+ Stimulus_Strength (`self.NoiseMeter`)))
  (`KismetSystemLibrary.PrintString` (`KismetStringLibrary.Conv_DoubleToString` (`self.NoiseMeter`)))
  (switch `/Game/Blueprints/Witch/E_WitchState` (`/Game/Blueprints/Witch/BP_WoodenWitch.State` (`self.Witch`))
    (:`NewEnumerator0`
      (if (>= (`self.NoiseMeter`) 0.0)
        (`/Game/Blueprints/Witch/BP_WoodenWitch.SwapState` (`self.Witch`) "NewEnumerator1")
        (`/Game/Blueprints/Witch/BP_WoodenWitch.ServerPlayMontage` (`self.Witch`) "/Game/Assets/Animations/AM_Witch_Lock_on_Montage.AM_Witch_Lock_on_Montage")))
    (:`NewEnumerator1`
      (if (>= (`self.NoiseMeter`) 10.0)
        (`/Game/Blueprints/Witch/BP_WoodenWitch.SwapState` (`self.Witch`) "NewEnumerator2")
        (`/Game/Blueprints/Witch/BP_WoodenWitch.ServerPlayMontage` (`self.Witch`) "/Game/Assets/Animations/AM_Witch_Shriek_Montage.AM_Witch_Shriek_Montage")
        (`BlackboardComponent.SetValueAsObject` (`AIBlueprintHelperLibrary.GetBlackboard` null) "TargetPlayer" Actor)))))

(event `ServerSetNoiseMeter`
  (params (NoiseStrenght :type "Float (double-precision)"))
  (`self.SetNoiseMeter` NoiseStrenght))

(event `SetNoiseMeter`
  (params (NoiseStrenght :type "Float (double-precision)"))
  (set `self.NoiseMeter` NoiseStrenght))

(fn `UserConstructionScript`)