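; BP_TestDoll is a test flammable doll that draws the wooden witch toward whoever sets it alight.
; On the first Ignite only, it activates Niagara and makes a noise at BP_WoodenWitch's location, instigated by the igniter.
; It writes the igniter's location directly to the witch's MoveLocation blackboard key and draws a debug sphere trace there.
; It reports a fixed flammable type, and its interact function is empty.
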(event `/Game/Blueprints/Management/BPI_Interract.Ignite`
  (params (Iginter :type "Pawn Object Reference"))
  (bind _returnvalue (`self.K2_GetActorLocation` Iginter))
  (`/Engine/EditorBlueprintResources/StandardMacros.DoOnce` false
    (:`Completed`
      (`ActorComponent.Activate` (`self.Niagara`) false)
      (bind _returnvalue_2 (`GameplayStatics.GetActorOfClass` "/Game/Blueprints/Witch/BP_WoodenWitch.BP_WoodenWitch_C"))
      (`self.MakeNoise` 3.0 Iginter (`self.K2_GetActorLocation` _returnvalue_2) 150.0)
      (`BlackboardComponent.SetValueAsVector` (`AIBlueprintHelperLibrary.GetBlackboard` _returnvalue_2) "MoveLocation" _returnvalue)
      (`KismetSystemLibrary.SphereTraceSingle` :`Start` _returnvalue :`End` _returnvalue :`Radius` 35.0 :`TraceChannel` "TraceTypeQuery1" :`DrawDebugType` "ForDuration"))))

(fn `GetFlamableType`
  (returns (Type :type "/Game/Blueprints/Management/E_FlameInterractable Enum"))
  (return "NewEnumerator2"))

(fn `Interract`
  (returns (Interractable :type "/Game/Blueprints/Interraction/BP_Interractable Object Reference"))
  (return null))

(fn `UserConstructionScript`)