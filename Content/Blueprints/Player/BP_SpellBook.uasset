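; BP_SpellBook holds the player's spell events: revive, freeze, unlock, deaf and blow, each gated by a spell count it never decrements.
; Most use TraceForSpell, a debug-drawn forward sphere trace, then filter hits by tag and cast.
; Only Unlock (toggles a door) and Blow (spawns a projectile) have effects; the others end at the cast.
; Deaf and Blow check ReviveSpellAmount, and Deaf traces zero distance.
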(event `RevieSpell`
  (params (Target :type "SceneComponent Object Reference"))
  (if (> (`self.ReviveSpellAmount`) 0)
    (bind _outhit (`self.TraceForSpell` Target 300.0 20.0))
    (bind (_bblockinghit _binitialoverlap _time _distance _location _impactpoint _normal _impactnormal _physmat _hitactor) (`GameplayStatics.BreakHitResult` _outhit))
    (if (`Actor.ActorHasTag` _hitactor "player")
      (cast `/Game/Blueprints/Player/BP_FirstPersonCharacter` _hitactor))))

(event `FreezeSpell`
  (params (Target :type "SceneComponent Object Reference"))
  (if (> (`self.FreezeSpellAmount`) 0)
    (bind _outhit (`self.TraceForSpell` Target 300.0 20.0))
    (bind (_bblockinghit _binitialoverlap _time _distance _location _impactpoint _normal _impactnormal _physmat _hitactor) (`GameplayStatics.BreakHitResult` _outhit))
    (if (`Actor.ActorHasTag` _hitactor "Witch")
      (cast `/Game/Blueprints/Witch/BP_WitchAiController` _hitactor))))

(event `UnlockSpell`
  (params (Target :type "SceneComponent Object Reference"))
  (if (> (`self.UnlockSpellAmount`) 0)
    (bind _outhit (`self.TraceForSpell` Target 300.0 20.0))
    (bind (_bblockinghit _binitialoverlap _time _distance _location _impactpoint _normal _impactnormal _physmat _hitactor) (`GameplayStatics.BreakHitResult` _outhit))
    (if (`Actor.ActorHasTag` _hitactor "Door")
      (bind _asbp_door (cast `/Game/Blueprints/Interraction/BP_Door` _hitactor))
      (`/Game/Blueprints/Interraction/BP_Door.Open/CloseDoor` _asbp_door))))

(event `DeafSpell`
  (params (InputPin :type "SceneComponent Object Reference"))
  (if (> (`self.ReviveSpellAmount`) 0)
    (bind _outhit (`self.TraceForSpell` InputPin 0.0 20.0))
    (bind (_bblockinghit _binitialoverlap _time _distance _location _impactpoint _normal _impactnormal _physmat _hitactor) (`GameplayStatics.BreakHitResult` _outhit))
    (if (`Actor.ActorHasTag` _hitactor "player")
      (cast `/Game/Blueprints/Player/BP_FirstPersonCharacter` _hitactor))))

(event `BlowSpell`
  (params (SpawnTransform :type "Transform Structure"))
  (if (> (`self.ReviveSpellAmount`) 0)
    (`|SpawnActorFromClass` "/Game/Blueprints/Spells/BlowProjectile.BlowProjectile_C" SpawnTransform "Undefined" "MultiplyWithRoot" null null)))

(fn `TraceForSpell`
  (params (Target :type "SceneComponent Object Reference") (TraceDistance :type "Float (single-precision)") (Radius :type "Float (single-precision)"))
  (returns (OutHit :type "HitResult Structure") (ReturnValue :type Boolean))
  (bind _returnvalue (`SceneComponent.K2_GetComponentLocation` Target))
  (bind (_outhit _returnvalue_2) (`KismetSystemLibrary.SphereTraceSingleForObjects` :`Start` _returnvalue :`End` (+ _returnvalue (* (`SceneComponent.GetForwardVector` Target) TraceDistance)) :`Radius` Radius :`ObjectTypes` (`|MakeArray` "ObjectTypeQuery1" "ObjectTypeQuery2" "ObjectTypeQuery4" "ObjectTypeQuery3" :!type "EObjectTypeQuery Enum") :`DrawDebugType` "ForDuration"))
  (return _outhit _returnvalue_2))