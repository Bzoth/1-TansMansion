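; Player spellbook component that pages through spell slots, acquires spells and casts them, clearing each slot after use.
; Page turns swap textures on dynamic page materials, with input locked during animations and actions routed through server/multicast-style events.
; For Revive and Unlock, a sphere trace highlights nearby tagged actors and a looping timer line-traces from the camera to select one.
; Revive and Unlock message that target, while Freeze spawns a projectile.
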(event `M_PrintSpell`
  (`KismetSystemLibrary.PrintString` (`|GetEnumeratorNameAsString` (`self.ActiveSpell`)) true true (struct :`R` 1.0 :`B` 0.667091 :`A` 1.0) 99999.0 (`KismetStringLibrary.Conv_StringToName` (`KismetStringLibrary.Concat_StrStr` (`KismetSystemLibrary.GetDisplayName` (`self.GetOwner`)) "Spell"))))

(event `EnhancedInput|/Game/Input/Actions/IA_NextSpell`
  (params (ActionValue :type Boolean) (ElapsedSeconds :type "Float (double-precision)") (TriggeredSeconds :type "Float (double-precision)") (InputAction :type "InputAction Object Reference" :default "/Game/Input/Actions/IA_NextSpell.IA_NextSpell"))
  (:`Started`
    (if (!= (`self.SpellIndex`) (- (`KismetArrayLibrary.Array_Length` (`self.Spells`)) 1))
      (if (`self.CanSwapPage`)
        (set `self.CanSwapPage` false)
        (`/Game/Blueprints/Player/BP_FirstPersonCharacter.S_NextSpellAnim` (`self.Player`))
        (`self.S_ChangePageMaterialsToNextPage`)))))

(event `S_ChangePageMaterialsToNextPage`
  (`self.M_ChangePageMaterialsToNextPage`))

(event `M_ChangePageMaterialsToNextPage`
  (`self.ChangePageMaterialsToNextPage`))

(event `ContinueOnChangePageMaterialsToNextPage`
  (bind _output_get (set `self.SpellIndex` (`KismetMathLibrary.Clamp` (+ (`self.SpellIndex`) 1) 0 (- (`KismetArrayLibrary.Array_Length` (`self.Spells`)) 1))))
  (set `self.ActiveSpell` (`|GetArrayItem` (`self.Spells`) _output_get))
  (`self.M_PrintSpell`)
  (`self.GetSpellTargetsNearby`)
  (set `self.WentNextPage` true))

(event `S_SetOverrideMaterial`
  (params (Target :type "Object Object Reference") (Override :type Boolean) (SelectedObject :type Boolean))
  (`self.C_SetOverrideMaterial` Target Override SelectedObject))

(event `self.ReceiveBeginPlay`
  (`|ExecutionSequence`
    (:`then_0`
      (`self.M_PrintSpell`))
    (:`then_1`
      (`self.M_CastToPlayer`))
    (:`then_2`
      (`KismetSystemLibrary.DelayUntilNextTick`)
      (`self.S_ChangePageMaterialsToNextPage`))))

(event `M_CastToPlayer`
  (bind _asbp_first_person_character (cast `/Game/Blueprints/Player/BP_FirstPersonCharacter` (`self.GetOwner`)))
  (`self.M_SetPlayer` _asbp_first_person_character))

(event `M_SetPlayer`
  (params (Player :type "/Game/Blueprints/Player/BP_FirstPersonCharacter Object Reference"))
  (set `self.Player` Player))

(event `C_SetOverrideMaterial`
  (params (Target :type "Object Object Reference") (Override :type Boolean) (SelectedObject :type Boolean))
  (message `/Game/Blueprints/Management/BPI_Interract.SetOverrideMaterial` Target Override SelectedObject))

(event `EnhancedInput|/Game/Input/Actions/IA_PreviousSpell`
  (params (ActionValue :type Boolean) (ElapsedSeconds :type "Float (double-precision)") (TriggeredSeconds :type "Float (double-precision)") (InputAction :type "InputAction Object Reference" :default "/Game/Input/Actions/IA_PreviousSpell.IA_PreviousSpell"))
  (:`Started`
    (if (!= (`self.SpellIndex`) 0)
      (if (`self.CanSwapPage`)
        (set `self.CanSwapPage` false)
        (`/Game/Blueprints/Player/BP_FirstPersonCharacter.S_PreviousSpellAnim` (`self.Player`))
        (`self.S_ChangePageMaterialsToPreviousPage`)))))

(event `S_ChangePageMaterialsToPreviousPage`
  (`self.M_ChangePageMaterialsToPreviousPage`))

(event `M_ChangePageMaterialsToPreviousPage`
  (`self.ChangePageMaterialsToPreviousPage`))

(event `ContinueOnChangePageMaterialsToPreviousPage`
  (bind _output_get (set `self.SpellIndex` (`KismetMathLibrary.Clamp` (- (`self.SpellIndex`) 1) 0 (- (`KismetArrayLibrary.Array_Length` (`self.Spells`)) 1))))
  (set `self.ActiveSpell` (`|GetArrayItem` (`self.Spells`) _output_get))
  (`self.M_PrintSpell`)
  (`self.GetSpellTargetsNearby`)
  (set `self.WentNextPage` false))

(event `M_SpellUsedOnTarget`
  (`self.SpellUsedOnTarget`))

(event `EnhancedInput|/Game/Input/Actions/IA_Shoot`
  (params (ActionValue :type Boolean) (ElapsedSeconds :type "Float (double-precision)") (TriggeredSeconds :type "Float (double-precision)") (InputAction :type "InputAction Object Reference" :default "/Game/Input/Actions/IA_Shoot.IA_Shoot"))
  (:`Started`
    (if (`|EnumInequality` (`self.ActiveSpell`) "NewEnumerator5")
      (if (`self.CanSwapPage`)
        (set `self.CanSwapPage` false)
        (`/Game/Blueprints/Player/BP_FirstPersonCharacter.S_SpellUsed` (`self.Player`))
        (`self.S_SpellUsedOnTarget`)))))

(event `S_SpellUsedOnTarget`
  (bind _player (`self.Player`))
  (bind _firstpersoncamera (`/Game/Blueprints/Player/BP_FirstPersonCharacter.FirstPersonCamera` (`self.Player`)))
  (bind (_returnvalue_location _returnvalue_rotation) (`KismetMathLibrary.BreakTransform` (`SceneComponent.K2_GetComponentToWorld` _firstpersoncamera)))
  (`self.M_SpellUsedOnTarget`)
  (switch `/Game/Blueprints/Player/E_Spells` (`self.ActiveSpell`)
    (:`NewEnumerator0`
      (message `/Game/Blueprints/Management/BPI_Interract.SpellCast` (`self.SpellTarget`) "NewEnumerator0"))
    (:`NewEnumerator1`
      (`|SpawnActorFromClass` "/Game/Blueprints/Spells/BP_ProjectileBase.BP_ProjectileBase_C" (`KismetMathLibrary.MakeTransform` (+ _returnvalue_location (* (`SceneComponent.GetForwardVector` _firstpersoncamera) 400.0)) _returnvalue_rotation) "AlwaysSpawn" "MultiplyWithRoot" _player _player null))))

(event `S_SpellCastFinished`
  (`self.M_SpellCastFinished`))

(event `M_SpellCastFinished`
  (bind _wentnextpage (`self.WentNextPage`))
  (bind _dynamicpages (`self.DynamicPages`))
  (set `self.CanSwapPage` true)
  (`MaterialInstanceDynamic.SetTextureParameterValue` (`|GetArrayItem` _dynamicpages (select `bool` _wentnextpage :`false` 1 :`true` 2)) "Spell_Texture" "/Game/Blueprints/Book/Materials/Textures/T_Page_Base.T_Page_Base")
  (`MaterialInstanceDynamic.SetTextureParameterValue` (`|GetArrayItem` _dynamicpages (select `bool` _wentnextpage :`true` 3)) "Spell_Texture" "/Game/Blueprints/Book/Materials/Textures/T_Page_Base.T_Page_Base")
  (`MaterialInstanceDynamic.SetScalarParameterValue` (`|GetArrayItem` _dynamicpages (select `bool` _wentnextpage :`true` 3)) "Rune_Opacity" 1.0)
  (`MaterialInstanceDynamic.SetScalarParameterValue` (`|GetArrayItem` _dynamicpages (select `bool` _wentnextpage :`false` 1 :`true` 2)) "Rune_Opacity" 1.0)
  (`KismetArrayLibrary.Array_Set` (`self.Spells`) (`self.SpellIndex`) "NewEnumerator5")
  (set `self.ActiveSpell` "NewEnumerator5")
  (`self.GetSpellTargetsNearby`))

(event `SpellAcquire`
  (params (SpellType :type "/Game/Blueprints/Player/E_Spells Enum" :default "NewEnumerator0"))
  (set `self.CanSwapPage` false)
  (`KismetArrayLibrary.Array_Set` (`self.Spells`) (`self.SpellIndex`) SpellType)
  (set `self.ActiveSpell` SpellType)
  (`MaterialInstanceDynamic.SetTextureParameterValue` (`|GetArrayItem` (`self.DynamicPages`) (select `bool` (`self.WentNextPage`) :`false` 1 :`true` 2)) "Spell_Texture" (select `/Game/Blueprints/Player/E_Spells` (`self.ActiveSpell`) :`NewEnumerator0` "/Game/Blueprints/Book/Materials/Textures/spells/reviveV2.reviveV2" :`NewEnumerator1` "/Game/Blueprints/Book/Materials/Textures/spells/freeze.freeze" :`NewEnumerator2` "/Game/Blueprints/Book/Materials/Textures/spells/unlock.unlock" :`NewEnumerator3` "/Game/Blueprints/Book/Materials/Textures/spells/blow.blow" :`NewEnumerator4` "/Game/Blueprints/Book/Materials/Textures/spells/deaf.deaf" :`NewEnumerator5` "/Game/Blueprints/Book/Materials/Textures/T_Page_Base.T_Page_Base" :!type "Texture Object Reference"))
  (`MaterialInstanceDynamic.SetTextureParameterValue` (`|GetArrayItem` (`self.DynamicPages`) (select `bool` (`self.WentNextPage`) :`true` 3)) "Spell_Texture" (select `/Game/Blueprints/Player/E_Spells` (`self.ActiveSpell`) :`NewEnumerator0` "/Game/Blueprints/Book/Materials/Textures/spells/reviveV2.reviveV2" :`NewEnumerator1` "/Game/Blueprints/Book/Materials/Textures/spells/freeze.freeze" :`NewEnumerator2` "/Game/Blueprints/Book/Materials/Textures/spells/unlock.unlock" :`NewEnumerator3` "/Game/Blueprints/Book/Materials/Textures/spells/blow.blow" :`NewEnumerator4` "/Game/Blueprints/Book/Materials/Textures/spells/deaf.deaf" :`NewEnumerator5` "/Game/Blueprints/Book/Materials/Textures/T_Page_Base.T_Page_Base" :!type "Texture Object Reference")))

(event `SpellCasted`
  (bind _spelltarget (`self.SpellTarget`))
  (switch `/Game/Blueprints/Player/E_Spells` (`self.ActiveSpell`)
    (:`NewEnumerator0`
      (`self.S_SetOverrideMaterial` (`self.SpellTarget`))
      (set `self.SpellTarget` null))
    (:`NewEnumerator2`
      (message `/Game/Blueprints/Management/BPI_Interract.SpellCast` _spelltarget "NewEnumerator2")
      (`self.S_SetOverrideMaterial` _spelltarget)
      (set `self.SpellTarget` null))))

(fn `ChangePageMaterialsToNextPage`
  (for (_array_element _array_index) (`self.DynamicPages`)
    (`MaterialInstanceDynamic.SetTextureParameterValue` _array_element "Spell_Texture" (select `bool` (<= _array_index 1) :`false` (select `bool` (!= (+ (`self.SpellIndex`) 1) (`KismetArrayLibrary.Array_Length` (`self.Spells`))) :`false` "/Game/Blueprints/Book/Materials/Textures/T_Page_Base.T_Page_Base" :`true` (select `/Game/Blueprints/Player/E_Spells` (`|GetArrayItem` (`self.Spells`) (+ (`self.SpellIndex`) 1)) :`NewEnumerator0` "/Game/Blueprints/Book/Materials/Textures/spells/reviveV2.reviveV2" :`NewEnumerator1` "/Game/Blueprints/Book/Materials/Textures/spells/freeze.freeze" :`NewEnumerator2` "/Game/Blueprints/Book/Materials/Textures/spells/unlock.unlock" :`NewEnumerator3` "/Game/Blueprints/Book/Materials/Textures/spells/blow.blow" :`NewEnumerator4` "/Game/Blueprints/Book/Materials/Textures/spells/deaf.deaf" :`NewEnumerator5` "/Game/Blueprints/Book/Materials/Textures/T_Page_Base.T_Page_Base" :!type "Texture Object Reference")) :`true` (select `/Game/Blueprints/Player/E_Spells` (`self.ActiveSpell`) :`NewEnumerator0` "/Game/Blueprints/Book/Materials/Textures/spells/reviveV2.reviveV2" :`NewEnumerator1` "/Game/Blueprints/Book/Materials/Textures/spells/freeze.freeze" :`NewEnumerator2` "/Game/Blueprints/Book/Materials/Textures/spells/unlock.unlock" :`NewEnumerator3` "/Game/Blueprints/Book/Materials/Textures/spells/blow.blow" :`NewEnumerator4` "/Game/Blueprints/Book/Materials/Textures/spells/deaf.deaf" :`NewEnumerator5` "/Game/Blueprints/Book/Materials/Textures/T_Page_Base.T_Page_Base" :!type "Texture Object Reference"))))
  (if (`self.InitialOpening`)
    (set `self.InitialOpening` false)
    (else
      (`self.ContinueOnChangePageMaterialsToNextPage`))))

(fn `ChangePageMaterialsToPreviousPage`
  (for (_array_element _array_index) (`self.DynamicPages`)
    (`MaterialInstanceDynamic.SetTextureParameterValue` _array_element "Spell_Texture" (select `bool` (>= _array_index 2) :`false` (select `bool` (!= (`self.SpellIndex`) 0) :`false` "/Game/Blueprints/Book/Materials/Textures/T_Page_Base.T_Page_Base" :`true` (select `/Game/Blueprints/Player/E_Spells` (`|GetArrayItem` (`self.Spells`) (- (`self.SpellIndex`) 1)) :`NewEnumerator0` "/Game/Blueprints/Book/Materials/Textures/spells/reviveV2.reviveV2" :`NewEnumerator1` "/Game/Blueprints/Book/Materials/Textures/spells/freeze.freeze" :`NewEnumerator2` "/Game/Blueprints/Book/Materials/Textures/spells/unlock.unlock" :`NewEnumerator3` "/Game/Blueprints/Book/Materials/Textures/spells/blow.blow" :`NewEnumerator4` "/Game/Blueprints/Book/Materials/Textures/spells/deaf.deaf" :`NewEnumerator5` "/Game/Blueprints/Book/Materials/Textures/T_Page_Base.T_Page_Base" :!type "Texture Object Reference")) :`true` (select `/Game/Blueprints/Player/E_Spells` (`self.ActiveSpell`) :`NewEnumerator0` "/Game/Blueprints/Book/Materials/Textures/spells/reviveV2.reviveV2" :`NewEnumerator1` "/Game/Blueprints/Book/Materials/Textures/spells/freeze.freeze" :`NewEnumerator2` "/Game/Blueprints/Book/Materials/Textures/spells/unlock.unlock" :`NewEnumerator3` "/Game/Blueprints/Book/Materials/Textures/spells/blow.blow" :`NewEnumerator4` "/Game/Blueprints/Book/Materials/Textures/spells/deaf.deaf" :`NewEnumerator5` "/Game/Blueprints/Book/Materials/Textures/T_Page_Base.T_Page_Base" :!type "Texture Object Reference"))))
  (`self.ContinueOnChangePageMaterialsToPreviousPage`))

(fn `GetSpellTargetsNearby`
  (bind (_origin _boxextent _sphereradius) (`KismetSystemLibrary.GetComponentBounds` (`/Game/Blueprints/Player/BP_FirstPersonCharacter.SpellSphere` (`self.Player`))))
  (for _array_element (`self.SpellTargets`)
    (`self.S_SetOverrideMaterial` _array_element))
  (`KismetArrayLibrary.Array_Clear` (`self.SpellTargets`))
  (bind _outhits (`KismetSystemLibrary.SphereTraceMultiForObjects` _origin _origin _sphereradius (`|MakeArray` "ObjectTypeQuery1" "ObjectTypeQuery2" "ObjectTypeQuery3" :!type "EObjectTypeQuery Enum")))
  (for _array_element_2 _outhits
    (bind (_bblockinghit _binitialoverlap _time _distance _location _impactpoint _normal _impactnormal _physmat _hitactor) (`GameplayStatics.BreakHitResult` _array_element_2))
    (if (`Actor.ActorHasTag` _hitactor (select `/Game/Blueprints/Player/E_Spells` (`self.ActiveSpell`) :`NewEnumerator0` "Revive" :`NewEnumerator2` "Unlock" :!type "Name"))
      (`KismetArrayLibrary.Array_Add` (`self.SpellTargets`) _hitactor)
      (`self.S_SetOverrideMaterial` _hitactor true)))
  (`self.StartSpellTargetTrace`))

(fn `SpellUsedOnTarget`
  (`KismetSystemLibrary.K2_ClearAndInvalidateTimerHandle` (`self.SpellTargetTimer`))
  (for _array_element (`self.SpellTargets`)
    (`self.S_SetOverrideMaterial` _array_element))
  (`KismetArrayLibrary.Array_Clear` (`self.SpellTargets`))
  (`self.S_SetOverrideMaterial` (`self.SpellTarget`) true true))

(fn `StartSpellTargetTrace`
  (`KismetSystemLibrary.K2_ClearAndInvalidateTimerHandle` (`self.SpellTargetTimer`))
  (if (or (`|EnumEquality` (`self.ActiveSpell`) "NewEnumerator0") (`|EnumEquality` (`self.ActiveSpell`) "NewEnumerator2"))
    (bind _returnvalue (`KismetSystemLibrary.K2_SetTimer` null "TraceForSelectedSpell" 0.01 true))
    (set `self.SpellTargetTimer` _returnvalue)))

(fn `TraceForSelectedSpell`
  (bind _player (`self.Player`))
  (bind _firstpersoncamera (`/Game/Blueprints/Player/BP_FirstPersonCharacter.FirstPersonCamera` _player))
  (bind _returnvalue (`SceneComponent.K2_GetComponentLocation` _firstpersoncamera))
  (bind _outhit (`KismetSystemLibrary.LineTraceSingle` _returnvalue (+ _returnvalue (* (`SceneComponent.GetForwardVector` _firstpersoncamera) (`.SphereRadius` (`KismetSystemLibrary.GetComponentBounds` (`/Game/Blueprints/Player/BP_FirstPersonCharacter.SpellSphere` _player))))) "TraceTypeQuery1"))
  (`self.S_SetOverrideMaterial` (`self.SpellTarget`) true)
  (bind (_bblockinghit _binitialoverlap _time _distance _location _impactpoint _normal _impactnormal _physmat _hitactor) (`GameplayStatics.BreakHitResult` _outhit))
  (`/Engine/EditorBlueprintResources/StandardMacros.IsValid` _hitactor
    (:`Is Valid`
      (if (`Actor.ActorHasTag` _hitactor (select `/Game/Blueprints/Player/E_Spells` (`self.ActiveSpell`) :`NewEnumerator0` "Revive" :`NewEnumerator2` "Unlock" :!type "Name"))
        (bind _output_get (set `self.SpellTarget` _hitactor))
        (`self.S_SetOverrideMaterial` _output_get true true)
        (else
          (set `self.SpellTarget` null)
          (`self.S_SetOverrideMaterial` _hitactor))))
    (:`Is Not Valid`
      (set `self.SpellTarget` null))))

(fn `TraceForSpell`
  (params (TraceDistance :type "Float (single-precision)") (Radius :type "Float (single-precision)") (Target :type "SceneComponent Object Reference"))
  (returns (OutHit :type "HitResult Structure") (ReturnValue :type Boolean))
  (bind _returnvalue (`SceneComponent.K2_GetComponentLocation` Target))
  (bind (_outhit _returnvalue_2) (`KismetSystemLibrary.SphereTraceSingleForObjects` :`Start` _returnvalue :`End` (+ _returnvalue (* (`SceneComponent.GetForwardVector` Target) TraceDistance)) :`Radius` Radius :`ObjectTypes` (`|MakeArray` "ObjectTypeQuery1" "ObjectTypeQuery2" "ObjectTypeQuery4" "ObjectTypeQuery3" :!type "EObjectTypeQuery Enum") :`DrawDebugType` "ForDuration"))
  (return _outhit _returnvalue_2))