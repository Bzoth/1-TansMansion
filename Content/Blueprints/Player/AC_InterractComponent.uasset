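; Player interaction component that picks up grabbable objects into an inventory and shows them in the right hand.
; IA_Interract triggers a camera-forward multi sphere trace, which interacts with the first tagged BP_Interractable found in Interractables.
; InterractWithObject stores "Grabable" results, copies their mesh to the hand and deactivates the actor.
; UseItem clears the hand mesh, reactivates the HandSlot item at the hand and removes it; RefreshHand is empty.
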(event `hebele`
  (`self.ReplicateTraceForInterect`))

(event `EnhancedInput|/Game/Input/Actions/IA_Interract`
  (params (ActionValue :type Boolean) (ElapsedSeconds :type "Float (double-precision)") (TriggeredSeconds :type "Float (double-precision)") (InputAction :type "InputAction Object Reference" :default "/Game/Input/Actions/IA_Interract.IA_Interract"))
  (:`Started`
    (`self.hebele`)))

(event `ReplicateTraceForInterect`
  (`self.TraceForInterract`))

(fn `InterractWithObject`
  (params (Interractable :type "Object Object Reference"))
  (`/Engine/EditorBlueprintResources/StandardMacros.IsValid` Interractable
    (:`Is Valid`
      (bind _interractable (message `/Game/Blueprints/Management/BPI_Interract.Interract` Interractable (`self.Player`)))
      (if (`Actor.ActorHasTag` _interractable "Grabable")
        (`KismetArrayLibrary.Array_Add` (`self.Inventory`) _interractable)
        (`StaticMeshComponent.SetStaticMesh` (`/Game/Blueprints/Player/BP_FirstPersonCharacter.RightHandMesh` (`self.Player`)) (`StaticMeshComponent.StaticMesh` (`/Game/Blueprints/Interraction/BP_Interractable.StaticMesh` _interractable)))
        (`/Game/Blueprints/Interraction/BP_Interractable.SetActorInUse` _interractable false (0.0 0.0 0.0))))))

(fn `RefreshHand`)

(fn `TraceForInterract`
  (bind _firstpersoncamera (`/Game/Blueprints/Player/BP_FirstPersonCharacter.FirstPersonCamera` (`self.Player`)))
  (bind _returnvalue (`SceneComponent.K2_GetComponentLocation` _firstpersoncamera))
  (bind _outhits (`KismetSystemLibrary.SphereTraceMultiForObjects` _returnvalue (+ _returnvalue (* (`SceneComponent.GetForwardVector` _firstpersoncamera) 300.0)) 20.0 (`|MakeArray` "ObjectTypeQuery1" "ObjectTypeQuery2" "ObjectTypeQuery4" "ObjectTypeQuery3" :!type "EObjectTypeQuery Enum")))
  (for _array_element _outhits
    (bind (_bblockinghit _binitialoverlap _time _distance _location _impactpoint _normal _impactnormal _physmat _hitactor _hitcomponent) (`GameplayStatics.BreakHitResult` _array_element))
    (if (`self.ComponentHasTag` _hitcomponent "Interractable")
      (bind _asbp_interractable (cast `/Game/Blueprints/Interraction/BP_Interractable` _hitactor))
      (if (`KismetArrayLibrary.Array_Contains` (`self.Interractables`) _asbp_interractable)
        (`self.InterractWithObject` _asbp_interractable)
        (break)))))

(fn `UseItem`
  (bind _inventory (`self.Inventory`))
  (bind _output (`|GetArrayItem` _inventory (`self.HandSlot`)))
  (if (`KismetArrayLibrary.Array_IsNotEmpty` (`self.Inventory`))
    (`StaticMeshComponent.SetStaticMesh` (`/Game/Blueprints/Player/BP_FirstPersonCharacter.RightHandMesh` (`self.Player`)) null)
    (`/Engine/EditorBlueprintResources/StandardMacros.IsValid` _output
      (:`Is Valid`
        (`/Game/Blueprints/Interraction/BP_Interractable.SetActorInUse` _output true (`SceneComponent.K2_GetComponentLocation` (`/Game/Blueprints/Player/BP_FirstPersonCharacter.RightHand` (`self.Player`))))
        (`KismetArrayLibrary.Array_RemoveItem` _inventory _output)))))