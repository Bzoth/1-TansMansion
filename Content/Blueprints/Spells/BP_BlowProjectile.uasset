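; BP_BlowProjectile is a spell projectile that delivers a blow effect to the actor it overlaps.
; On spawn, a timeline scales its sphere, then activates projectile movement, and a timer destroys it after a fixed lifetime.
; Overlap sends BlowTargetMessage with its location and destroys it; the OR-based Player/self filter also lets the player through.
; GetFlamableType returns a fixed enum value, and Interract is empty.
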(event `self.ReceiveBeginPlay`
  (`KismetSystemLibrary.K2_SetTimerDelegate` (delegate `DestroyProjetcile`) 5.0)
  (bind (_direction _newtrack_0) (`Timeline|TL_Begin` :!via `PlayFromStart`)
    (:`Update`
      (`SceneComponent.SetRelativeScale3D` (`self.Sphere`) (`KismetMathLibrary.Conv_DoubleToVector` _newtrack_0)))
    (:`Finished`
      (`ActorComponent.Activate` (`self.ProjectileMovement`) false))))

(event `DestroyProjetcile`
  (`self.K2_DestroyActor`))

(event `self.Sphere1.OnComponentBeginOverlap`
  (params (OverlappedComponent :type "PrimitiveComponent Object Reference") (OtherActor :type "Actor Object Reference") (OtherComp :type "PrimitiveComponent Object Reference") (OtherBodyIndex :type Integer) (bFromSweep :type Boolean) (SweepResult :type "HitResult Structure (by ref)"))
  (if (or (!= (`self.Player`) OtherActor) (!= self OtherActor))
    (message `/Game/Blueprints/Management/BPI_Interract.BlowTarget` OtherActor (`self.K2_GetActorLocation`))
    (`self.K2_DestroyActor`)))

(fn `GetFlamableType`
  (returns (Type :type "/Game/Blueprints/Management/E_FlameInterractable Enum"))
  (return "NewEnumerator2"))

(fn `Interract`
  (params (Interractor :type "Actor Object Reference"))
  (returns (Interractable :type "/Game/Blueprints/Interraction/BP_Interractable Object Reference"))
  (return null))

(fn `UserConstructionScript`)