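; BP_SpellTestDoor is a door actor, named as a spell test object, that opens when interacted with.
; Interract calls OpenDoor, which instantly adds 90 degrees to the mesh's world yaw on every call, with no closed state.
; GetFlamableType reports a fixed flammability enum value.
; SetOverrideMaterial always applies M_Overlay, ignoring its inputs because the material selection logic is left unconnected.
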(event `OpenDoor`
  (bind (_returnvalue_roll _returnvalue_pitch _returnvalue_yaw) (`KismetMathLibrary.BreakRotator` (`SceneComponent.K2_GetComponentRotation` (`self.StaticMesh`))))
  (`SceneComponent.K2_SetWorldRotation` (`self.StaticMesh`) (`KismetMathLibrary.MakeRotator` 0.0 0.0 (+ 90.0 _returnvalue_yaw)) false false))

(event `/Game/Blueprints/Management/BPI_Interract.SetOverrideMaterial`
  (params (Override :type Boolean) (SelectedObject :type Boolean))
  (`PrimitiveComponent.SetMaterial` (`self.StaticMesh`) 0 "/Game/Blueprints/Spells/M_Overlay.M_Overlay"))

(fn `GetFlamableType`
  (returns (Type :type "/Game/Blueprints/Management/E_FlameInterractable Enum"))
  (return "NewEnumerator2"))

(fn `Interract`
  (params (Interractor :type "Actor Object Reference"))
  (returns (Interractable :type "/Game/Blueprints/Interraction/BP_Interractable Object Reference"))
  (`self.OpenDoor`)
  (return null))

(fn `UserConstructionScript`)