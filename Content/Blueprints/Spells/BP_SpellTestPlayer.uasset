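; Test player actor for the spell system that reacts to spell casts and material-based selection highlighting.
; One spell type spawns a Niagara healing aura at the actor, which is deactivated after a short delay.
; SetOverrideMaterial swaps every static mesh slot between selected or plain overlay materials and the original per-slot character materials.
; It reports a fixed flammability type and leaves interaction empty.
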(event `M_DeactivateParticles`
  (params (Target :type "ActorComponent Object Reference"))
  (set `self.ReviveParticels` Target)
  (`KismetSystemLibrary.Delay` 3.0)
  (bind _reviveparticels (`self.ReviveParticels`)
    (:`then`
      (`ActorComponent.Deactivate` _reviveparticels))
    (:`else`)))

(event `/Game/Blueprints/Management/BPI_Interract.SpellCast`
  (params (Spell :type "/Game/Blueprints/Player/E_Spells Enum" :default "NewEnumerator0"))
  (if (`|EnumEquality` Spell "NewEnumerator0")
    (bind _returnvalue (`NiagaraFunctionLibrary.SpawnSystemAtLocation` "/Game/MixedVFX/Particles/Mix/NS_HealingAura.NS_HealingAura" (`self.K2_GetActorLocation`)))
    (`self.M_DeactivateParticles` _returnvalue)))

(event `/Game/Blueprints/Management/BPI_Interract.SetOverrideMaterial`
  (params (Override :type Boolean) (SelectedObject :type Boolean))
  (bind _staticmesh (`self.StaticMesh`))
  (for (_ _array_index) (`MeshComponent.GetMaterials` _staticmesh)
    (`PrimitiveComponent.SetMaterial` _staticmesh _array_index (select `bool` Override :`false` (select `int` _array_index :`0` "/Game/Blueprints/Player/Materials/MI_PC_CustomCoat.MI_PC_CustomCoat" :`1` "/Game/Blueprints/Player/Materials/M_PC_Default.M_PC_Default" :`2` "/Game/Blueprints/Player/Materials/M_PC_Face.M_PC_Face" :!type "MaterialInterface Object Reference") :`true` (select `bool` SelectedObject :`false` "/Game/Blueprints/Spells/M_Overlay.M_Overlay" :`true` "/Game/Blueprints/Spells/MI_OverlaySelected.MI_OverlaySelected" :!type "MaterialInterface Object Reference")))))

(fn `GetFlamableType`
  (returns (Type :type "/Game/Blueprints/Management/E_FlameInterractable Enum"))
  (return "NewEnumerator2"))

(fn `Interract`
  (params (Interractor :type "Actor Object Reference"))
  (returns (Interractable :type "/Game/Blueprints/Interraction/BP_Interractable Object Reference"))
  (return null))

(fn `UserConstructionScript`)