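; BP_Door is an interactable door that swings its frame mesh open or closed when Interract is called.
; It compares the interactor's position with the door's, using the actor's yaw to pick the world axis and sign for the swing direction.
; A timeline lerps the relative yaw, playing to open and reversing to close along the stored direction, with input locked until it finishes.
; Closed has an empty OnRep handler.
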(event `self.ReceiveBeginPlay`
  (`SceneComponent.K2_AttachToComponent` (`self.Widget`) (`self.SM_DoorFrame`) "None" "KeepRelative" "KeepRelative" "KeepRelative" true))

(event `Open/CloseDoor`
  (params (Interractor :type "Actor Object Reference"))
  (bind (_returnvalue_roll _returnvalue_pitch _returnvalue_yaw) (`KismetMathLibrary.BreakRotator` (`self.K2_GetActorRotation`)))
  (bind (_returnvalue_roll_2 _returnvalue_pitch_2 _returnvalue_yaw_2) (`KismetMathLibrary.BreakRotator` (`self.K2_GetActorRotation`)))
  (bind (_returnvalue_roll_3 _returnvalue_pitch_3 _returnvalue_yaw_3) (`KismetMathLibrary.BreakRotator` (`self.K2_GetActorRotation`)))
  (bind _returnvalue (`KismetMathLibrary.DegSin` _returnvalue_yaw_2))
  (bind _returnvalue_2 (select `bool` (== (== (`KismetMathLibrary.Abs` _returnvalue) _returnvalue) (<= (`KismetMathLibrary.Abs` (`KismetMathLibrary.DegSin` _returnvalue_yaw_3)) 0.1)) :`false` -1.0 :`true` 1.0))
  (if (`self.CanBeUsed`)
    (set `self.CanBeUsed` false)
    (set `self.Forward` (select `bool` (<= (`KismetMathLibrary.Abs` (`KismetMathLibrary.DegSin` _returnvalue_yaw)) 0.1) :`false` (> (.x (`self.K2_GetActorLocation` Interractor)) (.x (`self.K2_GetActorLocation`))) :`true` (> (.y (`self.K2_GetActorLocation` Interractor)) (.y (`self.K2_GetActorLocation`)))))
    (if (`self.Closed`)
      (set `self.Closed` false)
      (bind (_direction _doorrotation) (`Timeline|Door` :!label _label)
        (:`Update`
          (`SceneComponent.K2_SetRelativeRotation` (`self.SM_DoorFrame`) (`KismetMathLibrary.MakeRotator` 0.0 0.0 (`KismetMathLibrary.Lerp` 0.0 (select `bool` (`self.Closed`) :`false` (* (select `bool` (`self.Forward`) :`false` -160.0 :`true` 160.0) _returnvalue_2) :`true` (* (select `bool` (`self.OpenDirection`) :`false` -160.0 :`true` 160.0) _returnvalue_2)) _doorrotation)) false false))
        (:`Finished`
          (set `self.CanBeUsed` true)
          (set `self.OpenDirection` (`self.Forward`))))
      (else
        (set `self.Closed` true)
        (goto _label :!via `Reverse`)))))

(fn `Interract`
  (params (Interractor :type "Actor Object Reference"))
  (returns (Interractable :type "/Game/Blueprints/Interraction/BP_Interractable Object Reference"))
  (`self.Open/CloseDoor` Interractor)
  (return self))

(fn `OnRep_Closed`)

(fn `UserConstructionScript`
  (`parent.UserConstructionScript`))