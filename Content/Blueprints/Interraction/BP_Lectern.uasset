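; BP_Lectern is an interactable lectern that offers a spell scroll to the player, with its material set from SpellType in the construction script.
; Interract calls S_SpellTaken, which relays to M_SpellTaken, a naming pattern suggesting server-to-multicast replication.
; If a spell is available and the player's GetHasSpellMessage is false, it grants the spell and hides the scroll and widget.
; A timer later restores the scroll and availability, but not the widget.
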(event `M_SpellTaken`
  (params (Player :type "Actor Object Reference"))
  (if (`self.HasSpell`)
    (bind _hasspell (message `/Game/Blueprints/Management/BPI_Interract.GetHasSpell` Player))
    (if (not _hasspell)
      (message `/Game/Blueprints/Management/BPI_Interract.SpellAcquire` Player (`self.SpellType`))
      (set `self.HasSpell` false)
      (`SceneComponent.SetVisibility` (`self.StaticMesh1`) false false)
      (`SceneComponent.SetVisibility` (`self.Widget`) false false)
      (`KismetSystemLibrary.K2_SetTimerDelegate` (delegate `NewSpell`) 15.0))))

(event `S_SpellTaken`
  (params (Player :type "Actor Object Reference"))
  (`self.M_SpellTaken` Player))

(event `NewSpell`
  (`SceneComponent.SetVisibility` (`self.StaticMesh1`) true false)
  (set `self.HasSpell` true))

(fn `Interract`
  (params (Interractor :type "Actor Object Reference"))
  (returns (Interractable :type "/Game/Blueprints/Interraction/BP_Interractable Object Reference"))
  (`self.S_SpellTaken` Interractor)
  (return self))

(fn `UserConstructionScript`
  (`parent.UserConstructionScript`)
  (`PrimitiveComponent.SetMaterial` (`self.StaticMesh1`) 0 (select `/Game/Blueprints/Player/E_Spells` (`self.SpellType`) :`NewEnumerator0` "/Game/Blueprints/Book/Materials/MI_Spell_Scroll_Revive.MI_Spell_Scroll_Revive" :`NewEnumerator1` "/Game/Blueprints/Book/Materials/MI_Spell_Scroll_Freeze.MI_Spell_Scroll_Freeze" :`NewEnumerator2` "/Game/Blueprints/Book/Materials/MI_Spell_Scroll_Unlock.MI_Spell_Scroll_Unlock" :`NewEnumerator3` "/Game/Blueprints/Book/Materials/MI_Spell_Scroll_Blow.MI_Spell_Scroll_Blow" :`NewEnumerator4` "/Game/Blueprints/Book/Materials/MI_Spell_Book_Pages.MI_Spell_Book_Pages" :`NewEnumerator5` "/Game/Blueprints/Book/Materials/MI_Spell_Book_Pages.MI_Spell_Book_Pages" :!type "MaterialInterface Object Reference")))