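; BP_Interractable is an interactable actor that offers itself to the player on proximity, with an empty Interract function, likely for children to override.
; Unless Locked, sphere overlaps with Player-tagged components add or remove it from that actor's interactables and toggle its prompt widget, gated by CanBeInterracted.
; SetActorInUse toggles tick, collision and visibility and teleports it, suiting pooled reuse.
; GetFlamableType returns a fixed enum value.
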(event `self.SphereCollision.OnComponentBeginOverlap`
  (params (OverlappedComponent :type "PrimitiveComponent Object Reference") (OtherActor :type "Actor Object Reference") (OtherComp :type "PrimitiveComponent Object Reference") (OtherBodyIndex :type Integer) (bFromSweep :type Boolean) (SweepResult :type "HitResult Structure (by ref)"))
  (`/Engine/EditorBlueprintResources/StandardMacros.IsValid` OtherActor
    (:`Is Valid`
      (if (`ActorComponent.ComponentHasTag` OtherComp "Player")
        (if (not (`self.Locked`))
          (`self.SetCanBeInterractable` OtherActor true))))))

(event `self.SphereCollision.OnComponentEndOverlap`
  (params (OverlappedComponent :type "PrimitiveComponent Object Reference") (OtherActor :type "Actor Object Reference") (OtherComp :type "PrimitiveComponent Object Reference") (OtherBodyIndex :type Integer))
  (`/Engine/EditorBlueprintResources/StandardMacros.IsValid` OtherActor
    (:`Is Valid`
      (if (`ActorComponent.ComponentHasTag` OtherComp "Player")
        (if (not (`self.Locked`))
          (`self.SetCanBeInterractable` OtherActor))))))

(event `SetActorInUse`
  (params (InUse :type Boolean) (Location :type "Vector Structure"))
  (bind _inuse (`self.InUse`))
  (set `self.InUse` InUse)
  (`self.SetActorTickEnabled` _inuse)
  (`self.SetActorEnableCollision` _inuse)
  (`self.SetActorHiddenInGame` (not _inuse))
  (`self.K2_SetActorTransform` (`KismetMathLibrary.MakeTransform` Location (struct) (`SceneComponent.RelativeScale3D` (`self.StaticMesh`))) false true))

(fn `GetFlamableType`
  (returns (Type :type "/Game/Blueprints/Management/E_FlameInterractable Enum"))
  (return "NewEnumerator2"))

(fn `Interract`
  (params (Interractor :type "Actor Object Reference"))
  (returns (Interractable :type "/Game/Blueprints/Interraction/BP_Interractable Object Reference"))
  (return null))

(fn `SetCanBeInterractable`
  (params (OtherActor :type "Object Object Reference") (Value :type Boolean))
  (bind _otheractor (`local.OtherActor`))
  (bind _otheractor_2 (`local.OtherActor`))
  (if (`self.CanBeInterracted`)
    (if Value
      (message `/Game/Blueprints/Management/BPI_Interract.AddToInterractables` _otheractor_2 self)
      (message `/Game/Blueprints/Management/BPI_Interract.SetInterractWidget` _otheractor_2 (`self.Widget`) true)
      (else
        (message `/Game/Blueprints/Management/BPI_Interract.RemoveFromInterractables` _otheractor self)
        (bind _widget (`self.Widget`)
          (:`then`
            (message `/Game/Blueprints/Management/BPI_Interract.SetInterractWidget` _otheractor _widget false))
          (:`else`))))))

(fn `UserConstructionScript`)