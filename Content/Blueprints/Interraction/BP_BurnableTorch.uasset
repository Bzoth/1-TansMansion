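; BP_BurnableTorch is an interactable torch that can be set alight and reports a different flammable type once fully lit.
; Ignite routes through S_Ignite and M_Ignite events, named as a server-to-multicast chain, into IgniteFlames.
; IgniteFlames activates Niagara, hides the widget, disables interaction and starts a fast looping timer.
; The timer grows particle size through FirePower, then stops at a threshold and marks the torch as interacted.
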(event `self.ReceiveBeginPlay`)

(event `S_Ignite`
  (`self.M_Ignite`))

(event `M_Ignite`
  (`self.IgniteFlames`))

(event `/Game/Blueprints/Management/BPI_Interract.Ignite`
  (params (Iginter :type "Pawn Object Reference"))
  (`self.S_Ignite`))

(fn `Flames`
  (bind _result (`/Engine/EditorBlueprintResources/StandardMacros.IncrementFloat` (`self.FirePower`))
    (:`  `
      (`FXSystemComponent.SetFloatParameter` (`self.Niagara`) "Particle_Size" (/ _result 200.0))
      (if (>= (`self.FirePower`) 300.0)
        (`KismetSystemLibrary.K2_ClearAndInvalidateTimerHandle` (`self.FireTimer`))
        (set `self.Interracted` true)))))

(fn `GetFlamableType`
  (returns (Type :type "/Game/Blueprints/Management/E_FlameInterractable Enum"))
  (return (select `bool` (`self.Interracted`) :`false` "NewEnumerator1" :`true` "NewEnumerator2" :!type "/Game/Blueprints/Management/E_FlameInterractable Enum")))

(fn `IgniteFlames`
  (if (not (`self.Interracted`))
    (`ActorComponent.Activate` (`self.Niagara`) false)
    (bind _returnvalue (`KismetSystemLibrary.K2_SetTimer` null "Flames" 0.003 true))
    (set `self.FireTimer` _returnvalue)
    (`SceneComponent.SetVisibility` (`self.Widget`) false false)
    (set `self.CanBeInterracted` false)))

(fn `UserConstructionScript`)