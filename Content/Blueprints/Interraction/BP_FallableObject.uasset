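; BP_FallableObject is an interactable object that tips over when the player interacts with it and stops once it meets an obstacle.
; Interract starts a timeline that drives the pitch of the Scene component and removes the prompt widget and sphere collision on its first update.
; Each update also runs a debug-drawn sphere trace at Scene1 against WorldStatic objects, halting the timeline on a blocking hit with another actor.
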(event `DropFallableObject`
  (bind (_direction _newtrack_0) (`Timeline|FallAnim` :!label _label)
    (:`Update`
      (`SceneComponent.K2_SetRelativeRotation` (`self.Scene`) (`KismetMathLibrary.MakeRotator` 0.0 _newtrack_0) false false)
      (`self.TraceForStop`)
      (`/Engine/EditorBlueprintResources/StandardMacros.DoOnce` false
        (:`Completed`
          (`ActorComponent.K2_DestroyComponent` (`self.Widget`))
          (`ActorComponent.K2_DestroyComponent` (`self.SphereCollision`)))))))

(event `StopFallEvent`
  (goto _label :!via `Stop`))

(fn `Interract`
  (returns (Interractable :type "/Game/Blueprints/Interraction/BP_Interractable Object Reference"))
  (`self.DropFallableObject`)
  (return self))

(fn `TraceForStop`
  (bind _scene1 (`self.Scene1`))
  (bind (_returnvalue_x _returnvalue_y _returnvalue_z) (`KismetMathLibrary.BreakVector` (`SceneComponent.K2_GetComponentLocation` _scene1)))
  (bind _outhit (`KismetSystemLibrary.SphereTraceSingleForObjects` :`Start` (`SceneComponent.K2_GetComponentLocation` _scene1) :`End` (`KismetMathLibrary.MakeVector` (+ _returnvalue_x 5.0) _returnvalue_y _returnvalue_z) :`Radius` 20.0 :`ObjectTypes` (`|MakeArray` "ObjectTypeQuery1" :!type "EObjectTypeQuery Enum") :`DrawDebugType` "ForDuration"))
  (bind (_bblockinghit _binitialoverlap _time _distance _location _impactpoint _normal _impactnormal _physmat _hitactor) (`GameplayStatics.BreakHitResult` _outhit))
  (if (and _bblockinghit (!= _hitactor self))
    (`self.StopFallEvent`)))

(fn `UserConstructionScript`)