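; BP_RitualChamber is a ritual chamber Blueprint that burns candles in sequence in response to its dolls.
; On BeginPlay it passes its BurnCandel event to every entry in the Dolls array through AssignRitualDispatcher.
; Each BurnCandel call increments BurnedIndex, sets the candle at that index in Candels as burned, and prints its name and state.
; The index increments before use and has no bounds check.
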(event `self.ReceiveBeginPlay`
  (for _array_element (`self.Dolls`)
    (add `/Game/Blueprints/Interraction/BP_WitchDoll.RitualDispatcher` _array_element (delegate `BurnCandel`))))

(event `BurnCandel`
  (bind _output_get (set `self.BurnedIndex` (+ (`self.BurnedIndex`) 1)))
  (bind _output (`|GetArrayItem` (`self.Candels`) _output_get))
  (`/Game/Blueprints/Interraction/BP_RitualCandle.SetIsBurned` _output true)
  (`KismetSystemLibrary.PrintText` (`KismetTextLibrary.Conv_StringToText` (`KismetStringLibrary.Concat_StrStr` (`KismetSystemLibrary.GetDisplayName` _output) " " (`KismetStringLibrary.Conv_BoolToString` (`/Game/Blueprints/Interraction/BP_RitualCandle.IsBurned` _output))))))

(fn `UserConstructionScript`)