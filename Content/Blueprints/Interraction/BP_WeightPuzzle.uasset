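; BP_WeightPuzzle is an interactable puzzle actor that rotates its Cube once when triggered.
; Interract calls TriggerPuzzle, which sets IsSolved to block repeat triggers and plays a timeline that drives the cube's relative roll.
; It also reports a fixed flammable type through GetFlamableType; no weight check happens in this Blueprint.
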(event `TriggerPuzzle`
  (if (!= (`self.IsSolved`) true)
    (set `self.IsSolved` true)
    (bind (_direction _newtrack_0) (`Timeline|WeightPuzzleTimeline`)
      (:`Update`
        (`SceneComponent.K2_SetRelativeRotation` (`self.Cube`) (`KismetMathLibrary.MakeRotator` _newtrack_0) false false)))))

(fn `GetFlamableType`
  (returns (Type :type "/Game/Blueprints/Management/E_FlameInterractable Enum"))
  (return "NewEnumerator2"))

(fn `Interract`
  (returns (Interractable :type "/Game/Blueprints/Interraction/BP_Interractable Object Reference"))
  (`self.TriggerPuzzle`)
  (return self))

(fn `UserConstructionScript`)