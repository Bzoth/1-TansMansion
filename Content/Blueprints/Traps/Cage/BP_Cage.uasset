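; Cage trap actor with three padlocks that swings its door open once every lock is released.
; OpenLock takes a lock index and, gated by CanAction, plays a timeline that toggles that padlock's pitch in either direction.
; When it finishes, lock states are re-read from the pitches; if none remain locked, a DoOnce timeline rotates the door.
; Interract is empty and GetFlamableType returns a fixed type.
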(event `OpenLock`
  (params (Index :type Integer))
  (if (`self.CanAction`)
    (set `self.CanAction` false)
    (bind (_direction _newtrack_0) (`Timeline|TL_OpenLock` :!via `PlayFromStart`)
      (:`Update`
        (`self.SetLockRotation` _newtrack_0 Index))
      (:`Finished`
        (for (_array_element _array_index) (`|MakeArray` (`self.SM_LockPad1`) (`self.SM_LockPad2`) (`self.SM_LockPad3`))
          (bind (_relativerotation_roll _relativerotation_pitch) (`KismetMathLibrary.BreakRotator` (`SceneComponent.RelativeRotation` _array_element)))
          (`KismetArrayLibrary.Array_Set` (`self.Locks`) _array_index (< _relativerotation_pitch 30.0))
          (set `self.CanAction` true))
        (if (not (`KismetArrayLibrary.Array_Contains` (`self.Locks`) true))
          (`self.OpenCage`))))))

(event `OpenCage`
  (`/Engine/EditorBlueprintResources/StandardMacros.DoOnce` false
    (:`Completed`
      (bind (_direction _newtrack_0) (`Timeline|TL_OpenCage` :!via `PlayFromStart`)
        (:`Update`
          (`SceneComponent.K2_SetRelativeRotation` (`self.SM_Cage_Door`) (`KismetMathLibrary.MakeRotator` 0.0 0.0 _newtrack_0) false false))))))

(fn `GetFlamableType`
  (returns (Type :type "/Game/Blueprints/Management/E_FlameInterractable Enum"))
  (return "NewEnumerator2"))

(fn `Interract`
  (params (Interractor :type "Actor Object Reference"))
  (returns (Interractable :type "/Game/Blueprints/Interraction/BP_Interractable Object Reference"))
  (return null))

(fn `SetLockRotation`
  (params (Rotation :type "Float (single-precision)") (Index :type Integer))
  (`SceneComponent.K2_SetRelativeRotation` (select `int` (`local.Index`) :`0` (`self.SM_LockPad1`) :`1` (`self.SM_LockPad2`) :`2` (`self.SM_LockPad3`) :!type "SceneComponent Object Reference") (`KismetMathLibrary.MakeRotator` 0.0 (select `bool` (`|GetArrayItem` (`self.Locks`) (`local.Index`)) :`false` (- 45.0 (`local.Rotation`)) :`true` (`local.Rotation`) :!type "Float (single-precision)")) false false))

(fn `UserConstructionScript`)