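; An old clock actor that plays an idle sound and, when interacted with, switches to a trigger sound and emits a loud, long-range AI noise.
; Interract calls S-StartClock, which calls M_StartClock to swap the tracked audio cue with a short fade.
; The noise is instigated by the first BP_NoiseMaker found, using its forward vector as the noise location.
; BP_WoodenWitch overlapping SphereCollision switches the clock back to its idle sound.
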(event `1`
  (`self.2`))

(event `2`
  (bind _returnvalue (`GameplayStatics.SpawnSoundAtLocation` "/Game/Assets/Audio/SW_ClockIdle_Cue.SW_ClockIdle_Cue" (`self.K2_GetActorLocation`) (struct) 1.0 1.0 0.0 null null))
  (set `self.Cue` _returnvalue))

(event `self.ReceiveBeginPlay`
  (`self.1`))

(event `M_StartClock`
  (bind _cue (`self.Cue`))
  (`/Engine/EditorBlueprintResources/StandardMacros.IsValid` _cue
    (:`Is Valid`
      (`AudioComponent.FadeOut` _cue 0.1 0.0 "Linear")
      (bind _returnvalue (`GameplayStatics.SpawnSoundAtLocation` "/Game/Assets/Audio/SW_ClockTrigger_Cue.SW_ClockTrigger_Cue" (`self.K2_GetActorLocation`) (struct) 1.0 1.0 0.0 null null))
      (set `self.Cue` _returnvalue)
      (bind _returnvalue_2 (`GameplayStatics.GetActorOfClass` "/Game/Blueprints/Witch/BP_NoiseMaker.BP_NoiseMaker_C"))
      (`self.MakeNoise` 3.0 _returnvalue_2 (`self.GetActorForwardVector` _returnvalue_2) 360000.0))))

(event `S-StartClock`
  (`self.M_StartClock`))

(event `self.SphereCollision.OnComponentBeginOverlap`
  (params (OverlappedComponent :type "PrimitiveComponent Object Reference") (OtherActor :type "Actor Object Reference") (OtherComp :type "PrimitiveComponent Object Reference") (OtherBodyIndex :type Integer) (bFromSweep :type Boolean) (SweepResult :type "HitResult Structure (by ref)"))
  (bind _cue (`self.Cue`))
  (cast `/Game/Blueprints/Witch/BP_WoodenWitch` OtherActor)
  (`/Engine/EditorBlueprintResources/StandardMacros.IsValid` _cue
    (:`Is Valid`
      (`AudioComponent.FadeOut` _cue 0.1 0.0 "Linear")
      (bind _returnvalue (`GameplayStatics.SpawnSoundAtLocation` "/Game/Assets/Audio/SW_ClockIdle_Cue.SW_ClockIdle_Cue" (`self.K2_GetActorLocation`) (struct) 1.0 1.0 0.0 null null))
      (set `self.Cue` _returnvalue))))

(fn `Interract`
  (params (Interractor :type "Actor Object Reference"))
  (returns (Interractable :type "/Game/Blueprints/Interraction/BP_Interractable Object Reference"))
  (`self.S-StartClock`)
  (return self))

(fn `UserConstructionScript`)