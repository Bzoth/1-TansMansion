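; BP_SpellAcquire is a pickup that grants the player a spell of its configured SpellType.
; When a component tagged Player overlaps its Sphere, it sends SpellAcquireMessage with that type to the overlapping actor.
; The construction script creates a dynamic material on the Sphere and sets Spell_Texture to the image matching the spell type, so each placed instance shows its spell.
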(event `self.Sphere.OnComponentBeginOverlap`
  (params (OverlappedComponent :type "PrimitiveComponent Object Reference") (OtherActor :type "Actor Object Reference") (OtherComp :type "PrimitiveComponent Object Reference") (OtherBodyIndex :type Integer) (bFromSweep :type Boolean) (SweepResult :type "HitResult Structure (by ref)"))
  (`/Engine/EditorBlueprintResources/StandardMacros.IsValid` OtherActor
    (:`Is Valid`
      (if (`ActorComponent.ComponentHasTag` OtherComp "Player")
        (message `/Game/Blueprints/Management/BPI_Interract.SpellAcquire` OtherActor (`self.SpellType`))))))

(fn `UserConstructionScript`
  (bind _returnvalue (`PrimitiveComponent.CreateDynamicMaterialInstance` (`self.Sphere`) 0 null "None"))
  (`MaterialInstanceDynamic.SetTextureParameterValue` _returnvalue "Spell_Texture" (select `/Game/Blueprints/Player/E_Spells` (`self.SpellType`) :`NewEnumerator0` "/Game/Blueprints/Book/Materials/Textures/spells/reviveV2.reviveV2" :`NewEnumerator1` "/Game/Blueprints/Book/Materials/Textures/spells/freeze.freeze" :`NewEnumerator2` "/Game/Blueprints/Book/Materials/Textures/spells/unlock.unlock" :`NewEnumerator3` "/Game/Blueprints/Book/Materials/Textures/spells/blow.blow" :`NewEnumerator4` "/Game/Blueprints/Book/Materials/Textures/spells/deaf.deaf" :`NewEnumerator5` "/Game/Blueprints/Book/Materials/Textures/T_Page_Base.T_Page_Base" :!type "Texture Object Reference")))