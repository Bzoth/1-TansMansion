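; BP_Clock is an interactable clock actor that starts when its Interract function is called.
; Interract calls StartClock, which sets a one-second timer that spawns a sound at the world origin and plays a timeline from the start.
; The timeline drives the roll of the Scene component, and its Finished pin calls Play again, without rewinding.
; Print strings mark BeginPlay and interaction for debugging.
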(event `self.ReceiveBeginPlay`
  (`KismetSystemLibrary.PrintString` "Hello1"))

(event `StartClock`
  (`KismetSystemLibrary.PrintString` "Hello")
  (`KismetSystemLibrary.K2_SetTimerDelegate` (delegate `ClockTimer`) 1.0))

(event `StartTimeLineAgain`
  (bind (_direction _newtrack_0) (`Timeline|ClockTimeLine` :!label _label)
    (:`Update`
      (`SceneComponent.K2_SetRelativeRotation` (`self.Scene`) (`KismetMathLibrary.MakeRotator` _newtrack_0) false false))
    (:`Finished`
      (`self.StartTimeLineAgain`))))

(event `ClockTimer`
  (`GameplayStatics.SpawnSoundAtLocation` null (0.0 0.0 0.0) (struct) 1.0 1.0 0.0 null null)
  (goto _label :!via `PlayFromStart`))

(fn `Interract`
  (params (Interractor :type "Actor Object Reference"))
  (returns (Interractable :type "/Game/Blueprints/Interraction/BP_Interractable Object Reference"))
  (`KismetSystemLibrary.PrintString` "Hello3")
  (`self.StartClock`)
  (return self))

(fn `UserConstructionScript`
  (`parent.UserConstructionScript`))