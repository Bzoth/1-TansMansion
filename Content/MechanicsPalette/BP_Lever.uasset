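; BP_Lever is an interactable lever that unlocks a lock on a linked Cage.
; Interacting calls FlipLever, which, if the Cage is valid and allows action, opens the lock matching this lever's index.
; Each flip alternates a timeline forward or in reverse to rotate the handle mesh around its roll axis.
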(event `FlipLever`
  (`/Engine/EditorBlueprintResources/StandardMacros.IsValid` (`self.Cage`)
    (:`Is Valid`
      (if (`/Game/MechanicsPalette/BP_Cage.CanAction` (`self.Cage`))
        (`|ExecutionSequence`
          (:`then_0`
            (`/Game/MechanicsPalette/BP_Cage.OpenLock` (`self.Cage`) (`self.LeverIndex`)))
          (:`then_1`
            (`/Engine/EditorBlueprintResources/StandardMacros.FlipFlop`
              (:`A`
                (bind (_direction _newtrack_0) (`Timeline|TL_Lever` :!via `PlayFromStart` :!label _label)
                  (:`Update`
                    (`SceneComponent.K2_SetRelativeRotation` (`self.SM_Lever_Handle`) (`KismetMathLibrary.MakeRotator` _newtrack_0) false false))))
              (:`B`
                (goto _label :!via `ReverseFromEnd`)))))))))

(fn `Interract`
  (params (Interractor :type "Actor Object Reference"))
  (returns (Interractable :type "/Game/Blueprints/Interraction/BP_Interractable Object Reference"))
  (`self.FlipLever`)
  (return self))

(fn `UserConstructionScript`)